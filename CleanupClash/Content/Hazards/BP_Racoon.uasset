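; Raccoon hazard that attacks a player on contact, making them drop trash and stunning them.
; BeginPlay caches the player count and writes the spawn location and a cleared HasAttacked flag to the AI Blackboard.
; Sphere overlap matches the actor against each player, applies the attack and sets HasAttacked.
; Tick destroys the raccoon once it has attacked and is near its spawn point, a workaround for handling this outside the behavior tree.
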(event OnComponentBeginOverlap(Sphere)
  (params (OverlappedComponent :type Primitive%20Component%20Object%20Reference) (OtherActor :type Actor%20Object%20Reference) (OtherComp :type Primitive%20Component%20Object%20Reference) (OtherBodyIndex :type Integer) (bFromSweep :type Boolean) (SweepResult :type Hit%20Result%20Structure%20%28by%20ref%29))
  (for _index (range 0 (Variables|Default|GetPlayerLength))
    (if (== (Game|GetPlayerCharacter _index) OtherActor)
      (bind _output_get (Variables|Default|SetHasAttacked true))
      (AI|Components|Blackboard|SetValueasBool (AI|GetBlackboard 0) (Utilities|Name|MakeLiteralName "HasAttacked") _output_get)
      (bind _asplayer_character (Utilities|Casting|CastToPlayerCharacter (Game|GetPlayerCharacter _index)))
      (Class|PlayerCharacter|DropTrash _asplayer_character (* (Math|Vector|GetForwardVector (Transformation|GetActorRotation)) "-1.000000,-1.000000,1.000000"))
      (Class|PlayerCharacter|StunCharacter _asplayer_character))))

(event Custom|Die
  (Actor|DestroyActor))

(event EventBeginPlay
  (Utilities|FlowControl|Sequence
    (:then_0
      (bind _output_get (Variables|Default|SetHasAttacked false))
      (AI|Components|Blackboard|SetValueasBool (AI|GetBlackboard 0) (Utilities|Name|MakeLiteralName "HasAttacked") _output_get))
    (:then_1
      (bind _outactors (Actor|GetAllActorsOfClass "/Game/Player/BP_Player.BP_Player_C"))
      (Variables|Default|SetPlayerLength (Utilities|Array|Length _outactors)))
    (:then_2
      (bind _output_get_2 (Variables|Default|SetSpawnLocation (Transformation|GetWorldLocation (Variables|Collision|GetCapsuleComponent))))
      (AI|Components|Blackboard|SetValueasVector (AI|GetBlackboard 0) (Utilities|Name|MakeLiteralName "SpawnLocation") _output_get_2))))

(event EventTick
  (params (DeltaSeconds :type Float%20%28single-precision%29))
  (if (and (Utilities|Operators|EqualEqual (Transformation|GetActorLocation) (Variables|Default|GetSpawnLocation) 85.0) (Variables|Default|GetHasAttacked))
    (CallFunction|Die)))

(fn ConstructionScript)