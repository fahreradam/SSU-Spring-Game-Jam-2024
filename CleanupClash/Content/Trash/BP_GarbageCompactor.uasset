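; Garbage compactor actor that stores trash deposited by players and converts it into a summed value.
; Depositing moves a player's entire TrashArr into TrashArrCompactor.
; Compacting totals the stored elements, clears the array and returns the sum, while stealing moves only the last stored element to the player.
; The event graph is empty, so these functions rely on external callers.
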(event EventBeginPlay)

(event Collision|EventActorBeginOverlap
  (params (OtherActor :type Actor%20Object%20Reference)))

(event EventTick
  (params (DeltaSeconds :type Float%20%28single-precision%29)))

(fn ConstructionScript)

(fn OnPlayerAddTrash
  (params (player :type BP%20Player%20Object%20Reference))
  (bind _trasharr (Variables|/Game/Player/BP_Player.BP_Player_C|GetTrashArr player))
  (Utilities|Array|AppendArray (Variables|Default|GetTrashArrCompactor) _trasharr)
  (Utilities|Array|Clear _trasharr))

(fn OnPlayerCompactTrash
  (bind _trasharrcompactor (Variables|Default|GetTrashArrCompactor))
  (for _array_element _trasharrcompactor
    (LocalVariables|Setsum (+ (LocalVariables|Getsum) _array_element)))
  (Utilities|Array|Clear _trasharrcompactor)
  (return (LocalVariables|Getsum)))

(fn OnPlayerStealTrash
  (params (player :type BP%20Player%20Object%20Reference))
  (bind _trasharrcompactor (Variables|Default|GetTrashArrCompactor))
  (bind _returnvalue (Utilities|Array|Length _trasharrcompactor))
  (bind _returnvalue_2 (- _returnvalue 1))
  (Utilities|Array|Add (Variables|/Game/Player/BP_Player.BP_Player_C|GetTrashArr player) (Utilities|Array|Get(acopy) _trasharrcompactor _returnvalue_2))
  (Utilities|Array|RemoveIndex _trasharrcompactor _returnvalue_2))