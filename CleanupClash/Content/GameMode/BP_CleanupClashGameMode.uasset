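; Game mode for Cleanup Clash that sets up the match HUD and player start points.
; On BeginPlay it creates the game widget, adds it to the viewport, and assigns each garbage compactor to the widget's Team 1 or Team 2 slot by team name.
; The construction script caches all PlayerStart actors into StartPoints.
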(event EventBeginPlay
  (bind _returnvalue (UserInterface|CreateWidget "/Game/UI/GameWidget.GameWidget_C"))
  (UserInterface|Viewport|AddtoViewport _returnvalue 0)
  (bind _outactors (Actor|GetAllActorsOfClass "/Game/Trash/BP_GarbageCompactor.BP_GarbageCompactor_C"))
  (for _array_element _outactors
    (switch Utilities|FlowControl|Switch|SwitchonETeamName (Variables|/Game/Trash/BP_GarbageCompactor.BP_GarbageCompactor_C|GetTeamName _array_element)
      (:Team1
        (Variables|/Game/UI/GameWidget.GameWidget_C|SetTeam1Compactor _returnvalue _array_element))
      (:Team2
        (Variables|/Game/UI/GameWidget.GameWidget_C|SetTeam2Compactor _returnvalue _array_element)))))

(event EventTick
  (params (DeltaSeconds :type Float%20%28single-precision%29)))

(fn ConstructionScript
  (bind _outactors (Actor|GetAllActorsOfClass "/Script/Engine.PlayerStart"))
  (Variables|Default|SetStartPoints _outactors))